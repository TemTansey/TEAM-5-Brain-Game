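; RandItemBP spawns random physics-enabled item meshes at the level's SpawnPoint actors when play begins.
; Spawn creates a movable, simulated StaticMeshActor at each point's transform and assigns it a random mesh from StaticArray.
; Actors that receive a mesh are collected in ObjectOutputArray, then their mesh names are stored in Array and printed on screen.
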(event EventBeginPlay
  (bind _outactors (Actor|GetAllActorsOfClass "/Game/Brain_Game_Levels/Occipital_Lobe/SpawnPoint.SpawnPoint_C"))
  (bind _output_get (Variables|Default|SetSpawnLocations _outactors))
  (for _array_element _output_get
    (CallFunction|Spawn (Transformation|GetActorTransform _array_element)))
  (for _array_element_2 (Variables|Default|GetObjectOutputArray)
    (Utilities|Array|Add (Variables|Default|Getarray) (Utilities|GetObjectName (Variables|/Script/Engine.StaticMeshComponent|GetStaticMesh (Variables|/Script/Engine.StaticMeshActor|GetStaticMeshComponent _array_element_2))))
    (Development|PrintString (Utilities|GetObjectName (Variables|/Script/Engine.StaticMeshComponent|GetStaticMesh (Variables|/Script/Engine.StaticMeshActor|GetStaticMeshComponent _array_element_2))) true true "(R=0.000000,G=0.660000,B=1.000000,A=1.000000)" 2e+01)))

(fn ConstructionScript)

(fn Spawn
  (params (InputLocation :type Transform))
  ;[1 1 1] spawn random item
  (bind _returnvalue (Game|SpawnActorfromClass "/Script/Engine.StaticMeshActor" InputLocation "Undefined" 0 0))
  ;[1 1 1] Jack Murray Gay
  (Transformation|SetMobility (Variables|/Script/Engine.StaticMeshActor|GetStaticMeshComponent _returnvalue) "Movable")
  (Physics|SetSimulatePhysics (Variables|/Script/Engine.StaticMeshActor|GetStaticMeshComponent _returnvalue) true)
  (bind _returnvalue_2 (Components|StaticMesh|SetStaticMesh (Variables|/Script/Engine.StaticMeshActor|GetStaticMeshComponent _returnvalue) (.OutItem (Utilities|Array|Random (Variables|Default|GetStaticArray)))))
  (if _returnvalue_2
    (Utilities|Array|Add (Variables|Default|GetObjectOutputArray) _returnvalue)))